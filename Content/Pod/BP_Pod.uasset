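; Companion pod that hovers beside its owner, smoothly following per-state offsets and switching sides with the camera angle, and provides two weapons.
; The minigun fires pooled projectiles on a looping timer, aimed by a camera trace through a screen point.
; The charged cannon uses timers to briefly slow time, then trace, spawn a Chaos field at the impact and start a cooldown shown on a widget.
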(event Custom|ShowCircle
  (bind _alpha (Timeline|Timeline_ShowCircle PlayFromStart)
    (:Update
      (Rendering|Material|SetScalarParameterValue (Variables|FireMinigun|GetCircleDynamicMaterialInstance) "Step" _alpha :!class /Script/Engine.MaterialInstanceDynamic))))

(event Custom|HideCircle
  (bind _alpha (Timeline|Timeline_ShowCircle ReverseFromEnd)
    (:Update
      (Rendering|Material|SetScalarParameterValue (Variables|FireMinigun|GetCircleDynamicMaterialInstance) "Step" _alpha :!class /Script/Engine.MaterialInstanceDynamic))))

(event EventBeginPlay
  (FireMinigun|InitBulletPool)
  (bind _asbp_pod_player_controller (Utilities|Casting|CastToBP_PodPlayerController (Game|GetPlayerController 0)))
  (Variables|Default|SetPlayerController _asbp_pod_player_controller)
  (bind _aswbp_cooldown (Utilities|Casting|CastToWBP_Cooldown (UserInterface|GetWidget (Variables|Default|GetCooldownWidgetComp))))
  (bind _output_get (Variables|Default|SetCooldownWidget _aswbp_cooldown))
  (Variables|/Game/Pod/UI/WBP_Cooldown.WBP_Cooldown_C|SetPodOwner _output_get self)
  (bind _returnvalue (Rendering|Material|CreateDynamicMaterialInstance (Variables|Default|GetCircle) 0 0 "None" :!class /Script/Engine.PrimitiveComponent))
  (Variables|FireMinigun|SetCircleDynamicMaterialInstance _returnvalue))

(event Collision|EventActorBeginOverlap
  (params (OtherActor :type Actor%20Object%20Reference)))

(event EventTick
  (params (DeltaSeconds :type Float%20%28single-precision%29))
  (CallFunction|UpdateTransform DeltaSeconds))

(fn ConstructionScript)

(fn UpdateTransform
  (params (DeltaTime :type Float%20%28double-precision%29))
  (bind _podstate (CallFunction|GetCurrentState))
  (Transformation|SetActorLocationAndRotation (Math|Interpolation|VInterpTo (Transformation|GetActorLocation) (CallFunction|GetCurrentTargetLocation) DeltaTime (.interpspeed _podstate)) (Math|Interpolation|RInterpTo (Transformation|GetActorRotation) (CallFunction|GetCurrentTargetRotation) DeltaTime (.interpspeed _podstate))))

(fn SetState
  (params (NewActionState :type EPodActionState%20Enum :default "NewEnumerator0"))
  (Variables|Default|SetActionState NewActionState))

(fn GetCurrentState
  (return (.Value (Utilities|Map|Find (Variables|Default|GetStates) (Variables|Default|GetActionState)))))

(fn Init
  (Variables|Default|SetCameraComponent (Actor|GetComponentbyClass (Components|GetOwner) "/Script/Engine.CameraComponent"))
  (Transformation|SetActorLocationAndRotation (CallFunction|GetCurrentTargetLocation) (CallFunction|GetCurrentTargetRotation)))

(fn GetCurrentTargetLocation
  (bind _returnvalue (Components|GetOwner))
  (bind _actionstate (Variables|Default|GetActionState))
  (bind _cameracomponent (Variables|Default|GetCameraComponent))
  (bind _returnvalue_2 (Transformation|GetWorldTransform _cameracomponent))
  (bind _returnvalue_3 (Transformation|GetActorTransform _returnvalue))
  (bind _returnvalue_4 (Utilities|Enum|Equal(Enum) _actionstate "NewEnumerator2"))
  (bind _returnvalue_5 (select _returnvalue_4 _returnvalue_2 _returnvalue_3))
  (return (Math|Transform|TransformLocation _returnvalue_5 (+ (Math|Transform|InverseTransformLocation _returnvalue_5 (Transformation|GetActorLocation _returnvalue)) (CallFunction|ToSideLocation (.locationoffset (CallFunction|GetCurrentState)))))))

(fn GetCurrentTargetRotation
  (bind _podstate (CallFunction|GetCurrentState))
  (bind _worlddirection (CallFunction|ScreentoWorld 0.5 0.35))
  (bind _podstate_2 (CallFunction|GetCurrentState))
  (bind _cameracomponent (Variables|Default|GetCameraComponent))
  (bind _returnvalue (Transformation|GetWorldTransform _cameracomponent))
  (bind _returnvalue_2 (Transformation|GetWorldRotation _cameracomponent))
  (bind _roll (Math|Rotator|BreakRotator (.rotationoffset _podstate)))
  (bind _returnvalue_3 (Math|Rotator|MakeRotfromX _worlddirection))
  (bind _returnvalue_4 (Math|Transform|InverseTransformRotation _returnvalue _returnvalue_2))
  (bind _returnvalue_5 (Math|Rotator|CombineRotators _returnvalue_4 (.rotationoffset _podstate_2)))
  (bind _returnvalue_6 (Math|Transform|TransformRotation _returnvalue _returnvalue_5))
  (bind _returnvalue_7 (Math|Float|Clamp(Float) (.pitch _returnvalue_6) 0.0 1e+04))
  (bind _returnvalue_8 (Math|Rotator|MakeRotator _roll _returnvalue_7 (.yaw _returnvalue_6)))
  (return (Utilities|Select :Index (Variables|Default|GetActionState) :NewEnumerator0 _returnvalue_8 :NewEnumerator1 _returnvalue_3 :NewEnumerator3 _returnvalue_3 :NewEnumerator2 _returnvalue_8)))

(fn StartFireMinigun
  (if (Utilities|Enum|NotEqual(Enum) (Variables|Default|GetActionState) "NewEnumerator3")
    (CallFunction|SetState "NewEnumerator2")
    (Default|SetAimIconVisibility (Variables|Default|GetPlayerController) true)
    (CallFunction|ShowCircle)
    (Components|Activation|Activate (Variables|Default|GetMuzzleFlash) false)
    (bind _returnvalue (Utilities|Time|SetTimerbyFunctionName 0 "FireMinigun" (Variables|FireMinigun|GetFireRate) true))
    (Variables|FireMinigun|SetFireHandle _returnvalue)))

(fn StopFireMinigun
  (CallFunction|SetState "NewEnumerator0")
  (Default|SetAimIconVisibility (Variables|Default|GetPlayerController) false)
  (CallFunction|HideCircle)
  (Components|Activation|Deactivate (Variables|Default|GetMuzzleFlash))
  (Utilities|Time|ClearandInvalidateTimerbyHandle (Variables|FireMinigun|GetFireHandle)))

(fn StartFireCanon
  (if (and (not (Variables|FireCanon|GetInCooldown)) (Utilities|Enum|Equal(Enum) (Variables|Default|GetActionState) "NewEnumerator0"))
    (CallFunction|SetState "NewEnumerator3")
    (FireCanon|SetEmissiveFresnelEnabled true)
    (bind _returnvalue (Niagara|SpawnSystemAttached "/Game/Pod/VFX/NS_CanonLoad.NS_CanonLoad" (Variables|Default|GetSkeletalMesh) "ProjectileSocket" "0, 0, 0" "0, 0, 0" "SnapToTarget" false))
    (Variables|Default|SetFireCanonLoadingSystem _returnvalue)
    (bind _returnvalue_2 (Audio|SpawnSoundAttached "/Game/Pod/Sound/CanonLoadingLoop.CanonLoadingLoop" (Variables|Default|GetSkeletalMesh) "None" "0, 0, 0" "0, 0, 0" "KeepRelativeOffset" false 1.0 1.0 0.0 0 0))
    (Variables|FireCanon|SetFireCanonLoadingSound _returnvalue_2)
    (Audio|PlaySoundatLocation "/Game/Pod/Sound/CanonLoadingStart.CanonLoadingStart" (Transformation|GetActorLocation) "0, 0, 0" 1.0 1.0 0.0 0 0 0 0)
    (Rendering|SetVisibility (Variables|Default|GetLoadingWidgetComp) true false)
    (Default|SetAimIconVisibility (Variables|Default|GetPlayerController) true)))

(fn StopFireCanon
  (if (Utilities|Enum|Equal(Enum) (Variables|Default|GetActionState) "NewEnumerator3")
    (Components|Activation|Deactivate (Variables|Default|GetFireCanonLoadingSystem))
    (Audio|Components|Audio|FadeOut (Variables|FireCanon|GetFireCanonLoadingSound) 1.0 0.0 "Linear" :!class /Script/Engine.AudioComponent)
    (Utilities|Time|SetTimerbyFunctionName 0 "FireCanonStart" 0.1)))

(fn GetSide
  (bind _returnvalue (Components|GetOwner))
  (bind _cameracomponent (Variables|Default|GetCameraComponent))
  (bind _returnvalue_2 (Transformation|GetActorForwardVector _returnvalue))
  (bind _returnvalue_3 (Math|Vector|GetRightVector _cameracomponent))
  (bind _returnvalue_4 (Math|Vector|DotProduct _returnvalue_2 _returnvalue_3))
  (return (select (>= _returnvalue_4 0.0) "NewEnumerator0" "NewEnumerator1") _returnvalue_4))

(fn ToSideLocation
  (params (Location :type Vector))
  (bind (_result _dotvalue) (CallFunction|GetSide))
  (if (Utilities|Enum|Equal(Enum) _result (Variables|Default|GetSide))
    _
    (elif (Math|Boolean|ANDBoolean (> (Math|Float|Absolute(Float) _dotvalue) 0.2) (>= (Math|Vector|DotProduct (Transformation|GetActorForwardVector (Components|GetOwner)) (Math|Vector|GetForwardVector (Variables|Default|GetCameraComponent))) 0.0) (Utilities|Enum|NotEqual(Enum) (Variables|Default|GetActionState) "NewEnumerator2"))
      _
      (else
        ;[1 1 1] The side stay the same
        (return (CallFunction|GetSideLocation Location (Variables|Default|GetSide))))))
  ;[1 1 1] The side change
  (Variables|Default|SetSide _result)
  (return (CallFunction|GetSideLocation Location _result)))

(fn GetSideLocation
  (params (Location :type Vector) (Index :type EPodSide%20Enum :default "NewEnumerator0"))
  (bind (_x _y _z) (Math|Vector|BreakVector Location))
  (return (Utilities|Select :Index Index :NewEnumerator0 (Math|Vector|MakeVector _x (* _y -1.0) _z) :NewEnumerator1 Location)))

(fn FireMinigun
  (bind _bulletpool (Variables|FireMinigun|GetBulletPool))
  (bind _skeletalmesh (Variables|Default|GetSkeletalMesh))
  (bind _returnvalue (Transformation|GetSocketTransform _skeletalmesh "ProjectileSocket" "RTS_World"))
  ;[1 1 1] Get Projectile From Pool
  (if (> (Utilities|Array|Length _bulletpool) 0)
    (bind _output_get (LocalVariables|SetBullet (Utilities|Array|Get(acopy) _bulletpool)))
    (bind _returnvalue_2 (Utilities|Array|RemoveItem _bulletpool _output_get))
    (if _returnvalue_2
      ;[1 1 1] Trace from camera to target world location deprojected from screen location
      (bind (_outhit _returnvalue_3) (Collision|LineTraceByChannel (Transformation|GetWorldLocation (Variables|Default|GetCameraComponent)) (+ (* (CallFunction|ScreentoWorld (LocalVariables|GetTargetX) (LocalVariables|GetTargetY)) 1e+07) (Transformation|GetWorldLocation (Variables|Default|GetCameraComponent))) "TraceTypeQuery1" false 0 "None" true "(R=1.000000,G=0.000000,B=0.000000,A=1.000000)" "(R=0.000000,G=1.000000,B=0.000000,A=1.000000)" 3.0))
      ;[1 1 1] Launch projectile toward target location
      (if _returnvalue_3
        (bind (_tossvelocity _returnvalue_4) (Class|GameplayStatics|BlueprintSuggestProjectileVelocity (Transformation|GetSocketLocation (Variables|Default|GetSkeletalMesh) "ProjectileSocket") (.location _outhit) (Variables|FireMinigun|GetLaunchVelocity) 0.0 "DoNotTrace" 0.0 false false))
        (if _returnvalue_4
          (LocalVariables|SetLaunchDirection _tossvelocity)
          (else
            (LocalVariables|SetLaunchDirection (CallFunction|ScreentoWorld (LocalVariables|GetTargetX) (LocalVariables|GetTargetY)) :!label _label)))
        (else
          (goto _label)))
      (Default|Launch (LocalVariables|GetBullet) (LocalVariables|GetLaunchDirection) _returnvalue (Variables|FireMinigun|GetLaunchVelocity))
      (Audio|PlaySoundatLocation "/Game/Pod/Sound/FireMinigun_Cue.FireMinigun_Cue" (.Location (Math|Transform|BreakTransform _returnvalue)) "0, 0, 0" 1.0 1.0 0.0 "/Game/Pod/Sound/FireMinigun_Attenuation.FireMinigun_Attenuation" "/Game/Pod/Sound/FireMinigun_Concurrency.FireMinigun_Concurrency" 0 0))))

(fn InitBulletPool
  (for _index (range 0 (Variables|FireMinigun|GetBulletPoolSize))
    (bind _returnvalue (Game|SpawnActorfromClass "/Game/Pod/BP_PodProjectile.BP_PodProjectile_C" (Transformation|GetSocketTransform (Variables|Default|GetSkeletalMesh) "ProjectileSocket" "RTS_World") "AdjustIfPossibleButAlwaysSpawn" 0 0))
    (Utilities|Array|Add (Variables|FireMinigun|GetBulletPool) _returnvalue)
    (Rendering|SetVisibility (Variables|/Game/Pod/BP_PodProjectile.BP_PodProjectile_C|GetMesh _returnvalue) false false)
    (EventDispatchers|BindEventtoOnEnd _returnvalue (EventDispatchers|CreateEvent :!event AddBullettoPool))))

(fn AddBullettoPool
  (params (Bullet :type BP%20Pod%20Projectile%20Object%20Reference))
  (Utilities|Array|Add (Variables|FireMinigun|GetBulletPool) Bullet))

(fn ExitFireCanon
  (CallFunction|SetState "NewEnumerator0"))

(fn FireCanonStart
  (Utilities|Time|SetGlobalTimeDilation 0.6)
  (FireCanon|SetEmissiveFresnelEnabled false)
  (CallFunction|ShowCircle)
  (Rendering|SetVisibility (Variables|Default|GetLoadingWidgetComp) false false)
  (Audio|PlaySoundatLocation "/Game/Pod/Sound/FireCanon.FireCanon" (Transformation|GetActorLocation) "0, 0, 0" 1.0 1.0 0.0 0 0 0 0)
  (bind _returnvalue (Niagara|SpawnSystemAttached "/Game/Pod/VFX/NS_CanonFire.NS_CanonFire" (Variables|Default|GetSkeletalMesh) "ProjectileSocket" "0, 0, 0" "0, 0, 0" "KeepRelativeOffset" false))
  (Variables|Default|SetCanonFireSystem _returnvalue)
  (Utilities|Time|SetTimerbyFunctionName 0 "FireCanonEnd" 0.4))

(fn ScreentoWorld
  (params (TargetX :type Float%20%28double-precision%29) (TargetY :type Float%20%28double-precision%29))
  (bind _returnvalue (Game|GetPlayerController 0))
  (bind (_sizex _sizey) (HUD|GetViewportSize _returnvalue))
  (return (.WorldDirection (Class|GameplayStatics|DeprojectScreentoWorld _returnvalue (Math|Vector2D|MakeVector2D (* TargetX _sizex) (* TargetY _sizey))))))

(fn EndCooldown
  (Variables|FireCanon|SetInCooldown false)
  (Default|SetWidgetVisibility (Variables|Default|GetCooldownWidget) false))

(fn FireCanonEnd
  (bind _cameracomponent (Variables|Default|GetCameraComponent))
  (bind _returnvalue (Transformation|GetWorldLocation _cameracomponent))
  (Utilities|Time|SetGlobalTimeDilation 1.0)
  (Components|DestroyComponent (Variables|Default|GetFireCanonLoadingSystem))
  (bind (_outhit _returnvalue_2) (Collision|LineTraceByChannel _returnvalue (+ (* (CallFunction|ScreentoWorld (LocalVariables|GetTargetX) (LocalVariables|GetTargetY)) 1e+05) _returnvalue) "TraceTypeQuery1" false 0 "None" true "(R=1.000000,G=0.000000,B=0.000000,A=1.000000)" "(R=0.000000,G=1.000000,B=0.000000,A=1.000000)" 3.0))
  (if _returnvalue_2
    (CallFunction|SpawnChaosField (.Location (Collision|BreakHitResult _outhit)))
    (Effects|SpawnEmitteratLocation "/Game/Pod/VFX/P_CanonImpact.P_CanonImpact" (.Location (Collision|BreakHitResult _outhit))))
  (Default|SetAimIconVisibility (Variables|Default|GetPlayerController) false)
  (CallFunction|HideCircle)
  (Variables|FireCanon|SetInCooldown true)
  (Variables|FireCanon|SetCooldownStartTime (Utilities|Time|GetTimeSeconds))
  (Default|SetWidgetVisibility (Variables|Default|GetCooldownWidget) true)
  (Utilities|Time|SetTimerbyFunctionName 0 "ExitFireCanon" 0.8)
  (Utilities|Time|SetTimerbyFunctionName 0 "EndCooldown" (Variables|FireCanon|GetCooldownDuration)))

(fn GetCooldownPercent
  (return (Math|Float|Clamp(Float) (/ (- (Utilities|Time|GetTimeSeconds) (Variables|FireCanon|GetCooldownStartTime)) (Variables|FireCanon|GetCooldownDuration)))))

(fn GetCooldownRemainingDuration
  (return (Math|Integer|Clamp(Integer) (Math|Float|Truncate (* (- (Variables|FireCanon|GetCooldownDuration) (- (Utilities|Time|GetTimeSeconds) (Variables|FireCanon|GetCooldownStartTime))) 1e+02)) 0 100000000)))

(fn SetEmissiveFresnelEnabled
  (params (Enable :type Boolean))
  (bind _returnvalue (Rendering|Material|CreateDynamicMaterialInstance (Variables|Default|GetSkeletalMesh) 0 0 "None" :!class /Script/Engine.PrimitiveComponent))
  (Rendering|Material|SetScalarParameterValue _returnvalue "EnableFresnel" (Math|Float|SelectFloat 1.0 0.0 Enable) :!class /Script/Engine.MaterialInstanceDynamic))

(fn SpawnChaosField
  (params (SpawnTransform_Location :type Vector))
  (bind _returnvalue (Game|SpawnActorfromClass "/Engine/EditorResources/FieldNodes/FS_MasterField.FS_MasterField_C" (Math|Transform|MakeTransform SpawnTransform_Location "0, 0, 0" "0.700000,0.700000,7.000000") "Undefined" 0 0))
  (Variables|/Engine/EditorResources/FieldNodes/FS_MasterField.FS_MasterField_C|SetActivationType _returnvalue "NewEnumerator4")
  (Variables|/Engine/EditorResources/FieldNodes/FS_MasterField.FS_MasterField_C|SetFieldLifespan _returnvalue 0.1)
  (Variables|/Engine/EditorResources/FieldNodes/FS_MasterField.FS_MasterField_C|SetRadial%20Magnitude _returnvalue 1.5e+02)
  (Default|CETrigger _returnvalue))