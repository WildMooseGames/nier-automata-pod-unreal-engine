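; Reusable pod projectile that is launched and deactivated rather than destroyed.
; Launch places, shows and fires it along a direction, enabling collision after a short delay and starting a lifetime timer.
; On hit it plays impact effects and triggers a short-lived FS_MasterField at the impact, then ends.
; EndLaunch hides it, stops movement and collision, and calls OnEnd with itself.
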(event OnComponentHit(Mesh)
  (params (HitComponent :type Primitive%20Component%20Object%20Reference) (OtherActor :type Actor%20Object%20Reference) (OtherComp :type Primitive%20Component%20Object%20Reference) (NormalImpulse :type Vector :default "0, 0, 0") (Hit :type Hit%20Result%20Structure%20%28by%20ref%29))
  (bind (_bblockinghit _binitialoverlap _time _distance _location _impactpoint) (Collision|BreakHitResult Hit))
  (Effects|SpawnEmitteratLocation "/Game/Pod/VFX/P_Impact.P_Impact" _location)
  (Audio|PlaySoundatLocation "/Game/Pod/Sound/MinigunImpact_Cue.MinigunImpact_Cue" _location "0, 0, 0" 1.0 1.0 0.0 0 0 0 0)
  (bind _returnvalue (Game|SpawnActorfromClass "/Engine/EditorResources/FieldNodes/FS_MasterField.FS_MasterField_C" (Math|Transform|MakeTransform _location (.rotation (Math|Conversions|ToTransform(Vector) _impactpoint)) "0.500000,0.500000,0.500000") "Undefined" 0 0))
  (Variables|/Engine/EditorResources/FieldNodes/FS_MasterField.FS_MasterField_C|SetActivationType _returnvalue "NewEnumerator4")
  (Variables|/Engine/EditorResources/FieldNodes/FS_MasterField.FS_MasterField_C|SetFieldLifespan _returnvalue 0.1)
  (Variables|/Engine/EditorResources/FieldNodes/FS_MasterField.FS_MasterField_C|SetRadial%20Magnitude _returnvalue 1e+01)
  (Default|CETrigger _returnvalue)
  (CallFunction|EndLaunch))

(event EventBeginPlay)

(event Collision|EventActorBeginOverlap
  (params (OtherActor :type Actor%20Object%20Reference)))

(event EventTick
  (params (DeltaSeconds :type Float%20%28single-precision%29)))

(fn ConstructionScript)

(fn Launch
  (params (Direction :type Vector) (InitTransform :type Transform) (Velocity :type Float%20%28double-precision%29))
  (bind _projectilemovement (Variables|Default|GetProjectileMovement))
  (Transformation|SetActorTransform InitTransform)
  (Rendering|SetVisibility (Variables|Default|GetMesh) true false)
  (Transformation|SetActorRotation (Math|Rotator|MakeRotfromX Direction))
  (Components|Activation|Activate (Variables|Default|GetProjectileMovement) false)
  (Components|Movement|StopMovementImmediately _projectilemovement)
  (Game|Components|ProjectileMovement|SetVelocityinLocalSpace _projectilemovement (Math|Vector|MakeVector Velocity 0.0 0.0))
  (Variables|Default|SetIsLaunched true)
  (Utilities|Time|SetTimerbyFunctionName 0 "EnableProjectile" 0.03)
  (bind _returnvalue (Utilities|Time|SetTimerbyFunctionName 0 "EndLaunch" 3.0))
  (Variables|Default|SetEndLaunchTimer _returnvalue))

(fn EndLaunch
  (Rendering|SetVisibility (Variables|Default|GetMesh) false false)
  (Components|Activation|Deactivate (Variables|Default|GetProjectileMovement))
  (Variables|Default|SetIsLaunched false)
  (Collision|SetCollisionEnabled (Variables|Default|GetMesh) "NoCollision")
  (Utilities|Time|ClearandInvalidateTimerbyHandle (Variables|Default|GetEndLaunchTimer))
  (Default|CallOnEnd self))

(fn EnableProjectile
  (Collision|SetCollisionEnabled (Variables|Default|GetMesh) "QueryAndPhysics"))